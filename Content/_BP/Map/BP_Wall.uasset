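; BP_Wall is a map-building Blueprint that lays a wall mesh along an editable spline.
; The construction script adds one spline mesh component per segment, bent between neighboring points using their local positions and tangents, and assigns it the NewMesh mesh.
; Each component's relative location is also set to its segment's start point, on top of those local start and end positions.
; The event graph has no runtime logic.
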(event EventBeginPlay)

(event Collision|EventActorBeginOverlap
  (params (OtherActor :type Actor%20Object%20Reference)))

(event EventTick
  (params (DeltaSeconds :type Float%20%28single-precision%29)))

(fn ConstructionScript
  (bind _spline (Variables|Default|GetSpline))
  (bind _spline_2 (Variables|Default|GetSpline))
  (for _index (range 0 (- (Class|SplineComponent|GetNumberOfSplineSegments _spline) 1))
    (bind _returnvalue (AddComponent|AddSplineMeshComponent false (Math|Transform|MakeTransform (Spline|GetLocationatSplinePoint _spline _index "Local") "0, 0, 0" "1.000000,1.000000,1.000000")))
    (SplineMesh|SetStartandEnd _returnvalue (.Location (Spline|GetLocationandTangentatSplinePoint _spline_2 _index "Local")) (.Tangent (Spline|GetLocationandTangentatSplinePoint _spline_2 _index "Local")) (.Location (Spline|GetLocationandTangentatSplinePoint _spline_2 (+ _index 1) "Local")) (.Tangent (Spline|GetLocationandTangentatSplinePoint _spline_2 (+ _index 1) "Local")) true :!class /Script/Engine.SplineMeshComponent)
    (Components|StaticMesh|SetStaticMesh _returnvalue (Variables|Default|GetNew%20Mesh))))