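; Demo actor for the cel shader content that spins itself and cycles the color of the CelShadeLight actors attached to it.
; Each Tick it rotates around Axis by Speed per frame, without delta-time scaling.
; It advances a color vector at different per-channel rates over time, then wraps and normalizes it before setting it on each directly attached light.
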(event EventBeginPlay)

(event Collision|EventActorBeginOverlap
  (params (OtherActor :type Actor%20Object%20Reference)))

(event EventTick
  (params (DeltaSeconds :type Float%20%28single-precision%29))
  (Transformation|SetActorRotation (Math|Rotator|CombineRotators (Transformation|GetActorRotation) (Math|Vector|RotatorfromAxisandAngle (Variables|Default|GetAxis) (Variables|Default|GetSpeed))))
  (bind _output_get (Variables|Default|SetColor (+ (Variables|Default|GetColor) (* "0.100000,0.200000,0.300000" DeltaSeconds))))
  (for _array_element (Actor|GetAttachedActors true false)
    (bind _ascel_shade_light (Utilities|Casting|CastToCelShadeLight _array_element))
    (Variables|/Game/CelShader/CelShadeLight/Blueprints/CelShadeLight.CelShadeLight_C|SetColor _ascel_shade_light (Math|Conversions|ToColor(LinearColor) (Math|Conversions|ToLinearColor(Vector) (Math|Vector|Normalize (Math|Vector|MakeVector (Math|Float|Fraction (.X (Math|Vector|BreakVector _output_get))) (Math|Float|Fraction (.Y (Math|Vector|BreakVector _output_get))) (Math|Float|Fraction (.Z (Math|Vector|BreakVector _output_get))))))))))

(fn ConstructionScript)